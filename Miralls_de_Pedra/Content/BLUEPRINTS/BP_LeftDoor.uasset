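; BP_LeftDoor is an interactive left door, noted as the bell tower's, that the player opens and closes with E.
; Overlapping its box with the first-person character enables input and shows a prompt widget; leaving removes the widget but never disables input.
; Each E press flip-flops the OpenDoor timeline between play and reverse, lerping the door's yaw between closed and open angles.
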(event OnComponentBeginOverlap(Box)
  (params (OverlappedComponent :type Primitive%20Component%20Object%20Reference) (OtherActor :type Actor%20Object%20Reference) (OtherComp :type Primitive%20Component%20Object%20Reference) (OtherBodyIndex :type Integer) (bFromSweep :type Boolean) (SweepResult :type Hit%20Result%20Structure%20%28by%20ref%29))
  ;[0.15 0.15 0.15 0.5] Funcionament jugador-Porta campanar: al aproparse el jugador a la porta del campanar apareix un text abaix de la pantalla que permet premer la [E] i aixi poder entrar al interior
  ;;[0.15 0.15 0.15 0.5] Ha entrat a la caixa?
  ;;[0.15 0.15 0.15 0.5] El personatge ha entrat
  (Utilities|Casting|CastToBP_FirstPersonCharacter OtherActor)
  ;;[0.15 0.15 0.15 0.5] Permet utilitzar tecles dintre la caixa
  (Input|EnableInput (Game|GetPlayerController 0))
  ;;[0.15 0.15 0.15 0.5] S'ensenya la interficie
  (bind _returnvalue (UserInterface|CreateWidget "/Game/BLUEPRINTS/BP_UserInterfaceInteractionLeftDoor.BP_UserInterfaceInteractionLeftDoor_C"))
  (UserInterface|Viewport|AddtoViewport _returnvalue 0))

(event OnComponentEndOverlap(Box)
  (params (OverlappedComponent :type Primitive%20Component%20Object%20Reference) (OtherActor :type Actor%20Object%20Reference) (OtherComp :type Primitive%20Component%20Object%20Reference) (OtherBodyIndex :type Integer))
  ;[0.15 0.15 0.15 0.5] Funcionament jugador-Porta campanar: al aproparse el jugador a la porta del campanar apareix un text abaix de la pantalla que permet premer la [E] i aixi poder entrar al interior
  ;;[0.15 0.15 0.15 0.5] ha sortit de la caixa?
  ;;[0.15 0.15 0.15 0.5] El personatge ha sortit
  (Utilities|Casting|CastToBP_FirstPersonCharacter OtherActor)
  ;;[0.15 0.15 0.15 0.5] Es treu la interficie
  (Widget|RemovefromParent (stale OnComponentBeginOverlap(Box) _returnvalue)))

(event Input|KeyboardEvents|E
  (params (Key :type Key%20Structure :default "None"))
  ;[0.15 0.15 0.15 0.5] Funcionament jugador-Porta campanar: al aproparse el jugador a la porta del campanar apareix un text abaix de la pantalla que permet premer la [E] i aixi poder entrar al interior
  ;;[0.15 0.15 0.15 0.5] Al estar dintre de la caixa, es prem E i es carga el interior del campanar
  (:Pressed
    (Utilities|FlowControl|FlipFlop
      (:A
        (bind _animleftdoor (Timeline|Open%20Door Play)
          (:Update
            (Transformation|SetRelativeRotation (Variables|Default|GetDoor) (Math|Rotator|MakeRotator 0.0 0.0 (Math|Float|Lerp (Variables|Default|GetCloseLeftDoor) (Variables|Default|GetOpenLeftDoor) _animleftdoor)) false false))))
      (:B
        (Timeline|Open%20Door Reverse)))))

(fn ConstructionScript)